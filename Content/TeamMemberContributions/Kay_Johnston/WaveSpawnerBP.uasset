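; Wave spawner actor that creates batches of EnemyAI_KJ enemies at its own transform.
; On BeginPlay it registers SpawnEnemy with ThirdPersonGameMode's spawn-next-wave event, so the game mode drives wave timing.
; Each wave raises the next count by an increment that itself grows by one, so waves escalate faster than linearly.
; Spawns adjust to avoid collisions and are skipped when still blocked.
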(event Custom|SpawnEnemy
  (for _index (range 0 (- (Variables|Default|GetEnemySpawned) 1))
    (Game|SpawnActorfromClass "/Game/TeamMemberContributions/Kay_Johnston/EnemyAI_KJ.EnemyAI_KJ_C" (Transformation|GetActorTransform) "AdjustIfPossibleButDontSpawnIfColliding" 0 0))
  (Math|Integer|IncrementInt (Variables|Default|GetSpawnIncrement)
    (:%20%20
      (Variables|Default|SetEnemySpawned (+ (Variables|Default|GetEnemySpawned) (Variables|Default|GetSpawnIncrement))))))

(event EventBeginPlay
  (bind _asthird_person_game_mode (Utilities|Casting|CastToThirdPersonGameMode (Game|GetGameMode)))
  (EventDispatchers|BindEventtoSpawnNextWave _asthird_person_game_mode (delegate Custom|SpawnEnemy)))

(fn ConstructionScript)