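; Player controller Blueprint that opens and closes an in-game settings menu.
; The OpenSettingsMenu input creates a settings widget, adds it to the viewport, shows the cursor and sets Game and UI input focused on it with the mouse locked.
; The CloseWedigt event switches to game-only input and removes the widget, with the cursor flag still set to true.
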(event Custom|CloseWedigt
  (Variables|Default|SetbShowMouseCursor true)
  (Input|SetInputModeGameOnly self)
  (Widget|RemovefromParent (Variables|Default|GetSettingScreenRef)))

(event Input|ActionEvents|InputActionOpenSettingsMenu
  (params (Key :type Key%20Structure))
  (:Pressed
    (UserInterface|CreateWidget "/Game/TeamMemberContributions/Xuefei_Fu/Menu/OptionsInGame/WBP.WBP_C" self)
    (bind _output_get (Variables|Default|SetSettingScreenRef 0))
    (UserInterface|Viewport|AddtoViewport _output_get 0)
    (Variables|Default|SetbShowMouseCursor true)
    (Input|SetInputModeGameandUI self (Variables|Default|GetSettingScreenRef) "LockAlways" true)))

(fn ConstructionScript)